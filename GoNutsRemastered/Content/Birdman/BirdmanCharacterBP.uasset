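; Birdman AI character Blueprint that relays pursuit state to its behavior through the Blackboard.
; On BeginPlay it copies LaneY from the player's ThirdPersonCharacter, printing an error if that cast fails.
; OnEngagePursuit writes its IsInPursuit variable to the Blackboard, and OnPursuitCooldownOver sets the cooldown-over key to true.
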(event EventBeginPlay
  (bind _asthird_person_character (Utilities|Casting|CastToThirdPersonCharacter (Game|GetPlayerCharacter 0))
    (:then
      (Variables|Default|SetLaneY (Variables|/Game/ThirdPersonBP/Blueprints/ThirdPersonCharacter.ThirdPersonCharacter_C|GetLaneY _asthird_person_character)))
    (:CastFailed
      (Development|PrintString "Failed to find player character!" true true "(R=1.000000,G=0.000000,B=0.000000,A=1.000000)" 6.0))))

(event Collision|EventActorBeginOverlap
  (params (OtherActor :type Actor%20Object%20Reference)))

(event EventTick
  (params (DeltaSeconds :type Float%20%28single-precision%29)))

(event EventOnEngagePursuit
  (AI|Components|Blackboard|SetValueasBool (AI|GetBlackboard self) (Variables|Default|GetIsInPursuit) (Variables|Default|Get_isInPursuit)))

(event EventOnPursuitCooldownOver
  (AI|Components|Blackboard|SetValueasBool (AI|GetBlackboard 0) (Variables|Default|GetIsPursuitCooldownOver) true))

(fn ConstructionScript)