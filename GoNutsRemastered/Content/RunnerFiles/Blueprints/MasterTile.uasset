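; Endless-runner track tile that fills three lanes with random obstacles and keeps the run going.
; On BeginPlay, SpawnLane0 serves every lane, spawning a cone, spikes or empty placeholder actor, all destroyed after a fixed delay.
; When the character overlaps the Box, the game mode spawns another tile and adds multiplied points, walk speed rises within a clamp, and the tile later destroys itself.
; SpawnLane1, SpawnLane2 and a nested spawn chain are unused.
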(event OnComponentBeginOverlap(Box)
  (params (OverlappedComponent :type Primitive%20Component%20Object%20Reference) (OtherActor :type Actor%20Object%20Reference) (OtherComp :type Primitive%20Component%20Object%20Reference) (OtherBodyIndex :type Integer) (bFromSweep :type Boolean) (SweepResult :type Hit%20Result%20Structure%20%28by%20ref%29))
  (Utilities|Casting|CastToThirdPersonCharacter OtherActor)
  (bind _asthird_person_game_mode (Utilities|Casting|CastToThirdPersonGameMode (Game|GetGameMode)))
  (Default|SpawnTile _asthird_person_game_mode)
  (bind _asthird_person_game_mode_2 (Utilities|Casting|CastToThirdPersonGameMode (Game|GetGameMode)))
  (Variables|/Game/ThirdPersonBP/Blueprints/ThirdPersonGameMode.ThirdPersonGameMode_C|SetCurrentPoints _asthird_person_game_mode_2 (+ (* 1 (Variables|/Game/ThirdPersonBP/Blueprints/ThirdPersonGameMode.ThirdPersonGameMode_C|GetPointsMultiplier _asthird_person_game_mode_2)) (Variables|/Game/ThirdPersonBP/Blueprints/ThirdPersonGameMode.ThirdPersonGameMode_C|GetCurrentPoints _asthird_person_game_mode_2)))
  (bind _asthird_person_character (Utilities|Casting|CastToThirdPersonCharacter (Game|GetPlayerCharacter 0)))
  (Variables|/Script/Engine.CharacterMovementComponent|SetMaxWalkSpeed (Variables|/Script/Engine.Character|GetCharacterMovement _asthird_person_character) (Math|Float|Clamp(Float) (* (Variables|/Script/Engine.CharacterMovementComponent|GetMaxWalkSpeed (Variables|/Script/Engine.Character|GetCharacterMovement _asthird_person_character)) 1.01) 6e+02 1.2e+03))
  (Utilities|FlowControl|Delay 11.0)
  (Actor|DestroyActor))

(event EventBeginPlay
  (bind _obstacle_array (CallFunction|SpawnObstacles))
  (Utilities|FlowControl|Delay 1e+01)
  (Actor|DestroyActor _obstacle_array))

(event Collision|EventActorBeginOverlap
  (params (OtherActor :type Actor%20Object%20Reference)))

(event EventTick
  (params (DeltaSeconds :type Float%20%28single-precision%29)))

(fn ConstructionScript)

(fn SpawnObstacles
  (bind _actor (CallFunction|SpawnLane0 (Transformation|GetWorldTransform (Variables|Default|GetLane0))))
  (bind _actor_2 (CallFunction|SpawnLane0 (Transformation|GetWorldTransform (Variables|Default|GetLane1))))
  (bind _actor_3 (CallFunction|SpawnLane0 (Transformation|GetWorldTransform (Variables|Default|GetLane2))))
  (return (Utilities|Array|MakeArray _actor _actor_2 _actor_3)))

(fn SpawnLane0
  (params (NewParam :type Transform))
  (switch int (Math|Random|RandomIntegerinRange 0 3)
    (:0
      _)
    (:1
      (bind _returnvalue (Game|SpawnActorfromClass "/Game/RunnerFiles/Blueprints/Obstacle_Cone.Obstacle_Cone_C" NewParam "Undefined" 0 0))
      (return _returnvalue))
    (:2
      (bind _returnvalue_2 (Game|SpawnActorfromClass "/Game/RunnerFiles/Blueprints/Obstacle_Spikes.Obstacle_Spikes_C" NewParam "Undefined" 0 0))
      (return _returnvalue_2))
    (:3
      _))
  (bind _returnvalue_3 (Game|SpawnActorfromClass "/Script/Engine.Actor" (Variables|Default|GetZeroTransform) "Undefined" 0 0))
  (return _returnvalue_3))

(fn SpawnLane1
  (bind _lane1 (Variables|Default|GetLane1))
  (bind _returnvalue (Transformation|GetWorldTransform _lane1))
  (switch int (Math|Random|RandomIntegerinRange 0 3)
    (:1
      (Game|SpawnActorfromClass "/Game/RunnerFiles/Blueprints/Obstacle_Cone.Obstacle_Cone_C" _returnvalue "Undefined" 0 0))
    (:2
      (Game|SpawnActorfromClass "/Game/RunnerFiles/Blueprints/Obstacle_Spikes.Obstacle_Spikes_C" _returnvalue "Undefined" 0 0))))

(fn SpawnLane2
  (bind _lane2 (Variables|Default|GetLane2))
  (bind _returnvalue (Transformation|GetWorldTransform _lane2))
  (switch int (Math|Random|RandomIntegerinRange 0 3)
    (:1
      (Game|SpawnActorfromClass "/Game/RunnerFiles/Blueprints/Obstacle_Cone.Obstacle_Cone_C" _returnvalue "Undefined" 0 0))
    (:2
      (Game|SpawnActorfromClass "/Game/RunnerFiles/Blueprints/Obstacle_Spikes.Obstacle_Spikes_C" _returnvalue "Undefined" 0 0))))